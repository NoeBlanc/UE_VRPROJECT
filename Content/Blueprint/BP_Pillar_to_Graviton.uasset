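; BP_Pillar_to_Graviton is a pillar actor that teleports the player when a BP_MenuCube rests in its Start trigger.
; Beginning overlap starts a five-second one-shot timer, and ending overlap clears it, so removing the cube cancels the teleport.
; When the timer fires, player pawn 0 moves to the Cube component of the referenced REFTP actor, with rotation left unwired.
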(event OnComponentBeginOverlap(Start)
  (params (OverlappedComponent :type Primitive%20Component%20Object%20Reference) (OtherActor :type Actor%20Object%20Reference) (OtherComp :type Primitive%20Component%20Object%20Reference) (OtherBodyIndex :type Integer) (bFromSweep :type Boolean) (SweepResult :type Hit%20Result%20Structure%20%28by%20ref%29))
  (Utilities|Casting|CastToBP_MenuCube OtherActor)
  (bind _returnvalue (Utilities|Time|SetTimerbyEvent (delegate Custom|Teleport) 5.0)))

(event OnComponentEndOverlap(Start)
  (params (OverlappedComponent :type Primitive%20Component%20Object%20Reference) (OtherActor :type Actor%20Object%20Reference) (OtherComp :type Primitive%20Component%20Object%20Reference) (OtherBodyIndex :type Integer))
  (Utilities|Casting|CastToBP_MenuCube OtherActor)
  (Utilities|Time|ClearandInvalidateTimerbyHandle (stale OnComponentBeginOverlap(Start) _returnvalue)))

(event Custom|Teleport
  (Transformation|SetActorLocationAndRotation (Game|Player|GetPlayerPawn 0) (Transformation|GetWorldLocation (Variables|/Game/Blueprint/BP_TP_LocationRED.BP_TP_LocationRED_C|GetCube (Variables|Default|GetREF%20TP)))))

(event EventBeginPlay)

(event Collision|EventActorBeginOverlap
  (params (OtherActor :type Actor%20Object%20Reference)))

(event EventTick
  (params (DeltaSeconds :type Float%20%28single-precision%29)))

(fn ConstructionScript)