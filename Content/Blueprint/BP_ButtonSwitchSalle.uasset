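; BP_ButtonSwitchSalle is a VR button that teleports the player to another location, likely to switch rooms.
; When a component owned by a VRPawn overlaps its Box, ActivateButton sets the button's Cube to a lowered relative position, with no reset.
; It then moves player pawn 0 to the world location of the Cube in the referenced REFTP object.
; BeginPlay only runs a delay with nothing after it.
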(event OnComponentBeginOverlap(Box)
  (params (OverlappedComponent :type Primitive%20Component%20Object%20Reference) (OtherActor :type Actor%20Object%20Reference) (OtherComp :type Primitive%20Component%20Object%20Reference) (OtherBodyIndex :type Integer) (bFromSweep :type Boolean) (SweepResult :type Hit%20Result%20Structure%20%28by%20ref%29))
  (Utilities|Casting|CastToVRPawn (Components|GetOwner OtherComp))
  (CallFunction|ActivateButton)
  (Transformation|SetActorLocationAndRotation (Game|Player|GetPlayerPawn 0) (Transformation|GetWorldLocation (Variables|/Game/Blueprint/BP_TP_LocationRED.BP_TP_LocationRED_C|GetCube (Variables|Default|GetREF_TP)))))

(event EventBeginPlay
  (Utilities|FlowControl|Delay 2.0))

(event Collision|EventActorBeginOverlap
  (params (OtherActor :type Actor%20Object%20Reference)))

(event EventTick
  (params (DeltaSeconds :type Float%20%28single-precision%29)))

(fn ConstructionScript)

(fn ActivateButton
  (Transformation|SetRelativeLocation (Variables|Default|GetCube) "0.000000,0.000000,-50.000000" false false)
  (return))