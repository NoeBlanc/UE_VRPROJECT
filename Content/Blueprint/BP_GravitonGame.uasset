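; BP_GravitonGame is a puzzle manager Blueprint that decides whether a graviton game is solved.
; Its CheckSucces event loops over the Platform array and fails as soon as one platform's Success flag is false.
; When every platform succeeds, it makes the Succes component visible; both outcomes also print a debug string.
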(event Custom|CheckSucces
  (Variables|Default|SetFinish? true)
  (bind _array_element (Utilities|Array|ForEachLoopwithBreak (Variables|Default|GetPlatform) :!label _label)
    (:LoopBody
      (if (not (Variables|/Game/Blueprint/BP_PlatformGraviton.BP_PlatformGraviton_C|GetSuccess _array_element))
        (Variables|Default|SetFinish? false)
        (goto _label Break)))
    (:Completed
      (if (Variables|Default|GetFinish?)
        (Rendering|SetVisibility (Variables|Default|Getsucces) true false)
        (Development|PrintString "success")
        (else
          (Development|PrintString "NotYet"))))))

(fn ConstructionScript)