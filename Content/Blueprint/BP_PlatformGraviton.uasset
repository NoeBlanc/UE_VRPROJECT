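; BP_PlatformGraviton is a goal platform that tracks whether a graviton cube is resting on it.
; Its box overlap sets a Success flag when a BP_CubeGraviton enters and asks the Game reference to check for success.
; When the cube leaves, the flag is cleared and a debug "reseted" message prints.
; A disconnected delayed loop calling DesactivateMessage on array elements never runs.
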(event OnComponentBeginOverlap(Box)
  (params (OverlappedComponent :type Primitive%20Component%20Object%20Reference) (OtherActor :type Actor%20Object%20Reference) (OtherComp :type Primitive%20Component%20Object%20Reference) (OtherBodyIndex :type Integer) (bFromSweep :type Boolean) (SweepResult :type Hit%20Result%20Structure%20%28by%20ref%29))
  (Utilities|Casting|CastToBP_CubeGraviton OtherActor)
  (Variables|Default|SetSuccess true)
  (Default|CheckSucces (Variables|Default|GetGame)))

(event OnComponentEndOverlap(Box)
  (params (OverlappedComponent :type Primitive%20Component%20Object%20Reference) (OtherActor :type Actor%20Object%20Reference) (OtherComp :type Primitive%20Component%20Object%20Reference) (OtherBodyIndex :type Integer))
  (Utilities|Casting|CastToBP_CubeGraviton OtherActor)
  (Variables|Default|SetSuccess false)
  (Development|PrintString "reseted"))

(fn ConstructionScript)